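; Shields Up ability that gives the owning TestPTank a temporary shield actor when the ability action fires.
; It flags the tank's shield as active, spawns a ShieldsUpShield at the owner's location, passes it the shield duration, and stores it on the tank.
; The cast to TestPTank is marked as temporary, and nothing happens for other owner types.
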(event `self.AbilityAction`
  (bind _returnvalue (`self.GetOwner`))
  ;[1 1 1] TestPTank is TEMP
  (bind _astest_ptank (cast `/Game/Blueprints/Tanks/TestPTank` _returnvalue))
  (set `/Game/Blueprints/Tanks/TestPTank.Shield Active` true _astest_ptank)
  (bind _returnvalue_2 (`|SpawnActorFromClass` "/Game/Blueprints/Abilities/AbilityActors/ShieldsUpShield.ShieldsUpShield_C" (`KismetMathLibrary.Conv_VectorToTransform` (`Actor.K2_GetActorLocation` _returnvalue)) "Undefined" "OverrideRootScale" _returnvalue null))
  (set `/Game/Blueprints/Abilities/AbilityActors/ShieldsUpShield.Shield Duration` (`self.Shield Duration`) _returnvalue_2)
  (bind _astest_ptank_2 (cast `/Game/Blueprints/Tanks/TestPTank` (`self.GetOwner`)))
  (set `/Game/Blueprints/Tanks/TestPTank.Shield` _returnvalue_2 _astest_ptank_2))