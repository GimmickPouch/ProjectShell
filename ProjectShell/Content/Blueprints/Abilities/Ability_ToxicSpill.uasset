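; Toxic Spill tank ability that leaves a trail of toxic puddles beneath the owning tank.
; AbilityAction spawns puddles on a timed loop until the count limit, then waits and runs a destroy pass over the stored puddles.
; Damage is unfinished: TakeToxicDamage temporarily hurts the owner, the countdown events are empty, and the puddle-occupancy damage loop is disconnected.
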(event `Stop Toxic Countdown`
  ;[1 1 1] Broken AF - Stop Countdown
)

(event `Toxic Countdown to Damage`
  ;[1 0.2496 0.1498] Broken AF - Replace with tank taking damage immediately upon entering puddle, then 2 seconds later.
)

(event `self.AbilityAction`
  (bind _toxic_puddles (`self.Toxic Puddles`))
  (bind _toxic_puddles_2 (`self.Toxic Puddles`))
  ;[0.6963 1 0.7012] Spawn Puddles
  (`KismetSystemLibrary.Delay` (`self.Toxic Puddle Spawn Rate`) :!label _label)
  (bind _asbase_tank (cast `BaseTank` (`self.GetOwner`)))
  (bind _returnvalue (`|SpawnActorFromClass` "/Game/Blueprints/Abilities/AbilityActors/ToxicSpillPuddle.ToxicSpillPuddle_C" (`KismetMathLibrary.Conv_VectorToTransform` (`KismetMathLibrary.MakeVector` (.x (`Actor.K2_GetActorLocation` (`self.GetOwner`))) (.y (`Actor.K2_GetActorLocation` (`self.GetOwner`))) (- (.z (`Actor.K2_GetActorLocation` (`self.GetOwner`))) 30.0))) "Undefined" "OverrideRootScale" null _asbase_tank))
  (`KismetArrayLibrary.Array_Add` _toxic_puddles _returnvalue)
  (if (>= (`KismetArrayLibrary.Array_Length` _toxic_puddles) (`self.Number of Toxic Spill Puddles`))
    (`KismetSystemLibrary.Delay` (`self.Toxic Puddle Despawn Delay`))
    (for _array_element _toxic_puddles_2 :!label _label_2
      (`Actor.K2_DestroyActor` _array_element)
      (`KismetArrayLibrary.Array_RemoveItem` _toxic_puddles_2))
    (else
      (`self.Spawn Toxic Spill Puddle`))))

(event `Spawn Toxic Spill Puddle`
  ;[0.6963 1 0.7012] Spawn Puddles
  (goto _label))

(event `Remove ToxicSpill Puddles`
  ;[0.6963 1 0.7012] Spawn Puddles
  (goto _label_2))

(event `Take Toxic Damage`
  (bind _returnvalue (`self.GetOwner`))
  ;[0 1 0.2362] Take Toxic Damage
  (bind _asbase_tank (cast `BaseTank` _returnvalue))
  (bind _returnvalue_2 (`HealthComponent.TakeDamageAndCheckDeath` (`BaseTank.GetHealthComponent` _asbase_tank) 1.0))
  (if _returnvalue_2
    (`Actor.K2_DestroyActor` _returnvalue)))