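; Blink ability that teleports the owning BaseTank forward along its facing by TeleportRange.
; AbilityAction plays a charged or immediate sound, optionally delaying first, then nudges the tank upward and calls Teleport.
; An optional reappearance phase briefly disables input and query collision and zeroes MoveSpeed, which is never restored here.
; That phase is unfinished: re-enabling input is marked broken, the tank is never hidden, and VFX is only a placeholder.
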(event `self.AbilityAction`
  ;[1 1 1] Blink
  (bind _asbase_tank (cast `BaseTank` (`self.GetOwner`)))
  (`KismetSystemLibrary.PrintString` "Teleport Activated...")
  (if (`self.Enable Delayed Teleport`)
    (bind _returnvalue (+ (`Actor.K2_GetActorLocation` _asbase_tank) (0.0 0.0 1.0)))
    (`GameplayStatics.PlaySoundAtLocation` "/Game/Audio/Player/Tank/Abilities/Blink/Cue_TankBlinkCharge.Cue_TankBlinkCharge" _returnvalue)
    (`KismetSystemLibrary.Delay` 0.5)
    (else
      (`GameplayStatics.PlaySoundAtLocation` "/Game/Audio/Player/Tank/Abilities/Blink/Cut_TankBlinkImmediate.Cut_TankBlinkImmediate" _returnvalue)))
  (`Actor.K2_SetActorRelativeLocation` _asbase_tank _returnvalue false true)
  (bind _returnvalue_2 (`Actor.K2_TeleportTo` _asbase_tank (+ (`Actor.K2_GetActorLocation` _asbase_tank) (* (`Actor.GetActorForwardVector` _asbase_tank) (`self.Teleport Range`))) (`Actor.K2_GetActorRotation` _asbase_tank)))
  (if _returnvalue_2
    ;[1 1 1] Space for Unused VFX
    (`KismetSystemLibrary.PrintString` "VFX splash!")
    ;[1 1 1] Toggleable Delayed Reappearance Following Blink
    (if (`self.Enable Delayed Reappearance`)
      (`Actor.DisableInput` _asbase_tank null)
      (set `BaseTank.MoveSpeed` 0.0 _asbase_tank)
      (`Actor.SetActorHiddenInGame` _asbase_tank false)
      (`PrimitiveComponent.SetCollisionEnabled` (`BaseTank.TankMainBodyMesh` _asbase_tank) "PhysicsOnly")
      (`KismetSystemLibrary.Delay` 0.2)
      (bind _asbase_tank_2 (cast `BaseTank` (`self.GetOwner`)))
      ;;[1 1 1] Broken - Requires a Player Index
      (`Actor.EnableInput` _asbase_tank_2 null)
      (`Actor.SetActorHiddenInGame` _asbase_tank_2 false)
      (`PrimitiveComponent.SetCollisionEnabled` (`BaseTank.TankMainBodyMesh` _asbase_tank_2) "QueryAndPhysics"))
    (else
      (`KismetSystemLibrary.PrintString` "Blink Failed"))))