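; Tank ability component that lays a trail of oil spill puddles beneath its owning tank and slows tanks that drive into them.
; Activation spawns puddles on a short recursive delay until a maximum count, then destroys them all after a despawn delay.
; Puddle overlaps divide the tank's move speed, based on the owner's speed cached at BeginPlay.
; On exit, that cached speed returns only if no active puddle still overlaps the tank.
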(event `self.ReceiveBeginPlay`
  ;[1 1 1] Set Original Tank Move Speed
  (bind _asbase_tank (cast `BaseTank` (`self.GetOwner`)))
  (set `self.Original Tank Move Speed` (`BaseTank.MoveSpeed` _asbase_tank)))

(event `Spawn Oil Spill Puddle`
  (bind _active_puddles (`self.Active Puddles`))
  ;[0.09792 0.1406 0.0986] Spawn Puddle
  (`KismetSystemLibrary.Delay` 0.2)
  (bind _returnvalue (`|SpawnActorFromClass` "/Game/Blueprints/Abilities/AbilityActors/OilSpillPuddle.OilSpillPuddle_C" (`KismetMathLibrary.Conv_VectorToTransform` (`KismetMathLibrary.MakeVector` (.x (`Actor.K2_GetActorLocation` (`self.GetOwner`))) (.y (`Actor.K2_GetActorLocation` (`self.GetOwner`))) (- (.z (`Actor.K2_GetActorLocation` (`self.GetOwner`))) 30.0))) "Undefined" "OverrideRootScale" (stale `self.AbilityAction` _asbase_tank) null :!label _label))
  (`KismetArrayLibrary.Array_Add` (`self.Active Puddles`) _returnvalue)
  (if (== (`KismetArrayLibrary.Array_Length` (`self.Active Puddles`)) (`self.Maximum Number of Puddles`))
    (`KismetSystemLibrary.Delay` (`self.Oil Puddle Despawn Delay`))
    (for _array_element _active_puddles
      (`Actor.K2_DestroyActor` _array_element))
    (`KismetArrayLibrary.Array_Clear` _active_puddles)
    (else
      (`self.Spawn Oil Spill Puddle`))))

(event `self.AbilityAction`
  ;[0.09792 0.1406 0.0986] Spawn Puddle
  (bind _asbase_tank (cast `BaseTank` (`self.GetOwner`)))
  (goto _label))

(event `Tank Enters Puddle`
  (params (Tank :type "BaseTank Object Reference"))
  ;[1 1 1] Tank Enters Puddle, Called by Puddle Overlap
  (set `BaseTank.MoveSpeed` (/ (`self.Original Tank Move Speed`) (`self.Tank Movement Division`)) Tank))

(fn `TankLeavesPuddle`
  (params (Tank :type "BaseTank Object Reference"))
  (locals (TankIsFree :type Boolean :default true))
  (bind _active_puddles (`self.Active Puddles`))
  ;[1 1 1] Tank Leaves Puddle, Called by Puddle End Overlap
  (if (!= (`KismetArrayLibrary.Array_Length` _active_puddles) 0)
    (for _array_element _active_puddles
      (if (`KismetArrayLibrary.Array_Contains` (`/Game/Blueprints/Abilities/AbilityActors/OilSpillPuddle.Overlapping Tanks` _array_element) Tank)
        (set `local.TankIsFree` false)
        (break))))
  (if (`local.TankIsFree`)
    (set `BaseTank.MoveSpeed` (`self.Original Tank Move Speed`) Tank)))