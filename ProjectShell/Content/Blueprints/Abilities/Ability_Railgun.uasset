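; Railgun tank ability that fires a charged beam from the owning tank's cannon and damages the tank it hits.
; AbilityAction plays the fire sound, waits out the charge-up, then spawns a beam emitter at the cannon.
; A forward capsule trace on the Visibility channel shortens the beam to any impact point.
; A hit on the temporary TestPTank class applies damage, updates damage states and checks death, with optional debug prints.
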(event `self.AbilityAction`
  (bind _returnvalue (or (`self.Print Tank Damage Trace Hits`) (`self.Print All Trace Hits`)))
  ;[1 1 1] Railgun!
  ;;[0.4938 1 0.4158] Ability Action Plays Audio and Spawns VFX
  (bind _asbase_tank (cast `BaseTank` (`self.GetOwner`)))
  (bind _cannonstaticmesh (`BaseTank.CannonStaticMesh` _asbase_tank))
  (`GameplayStatics.SpawnSoundAttached` "/Game/Audio/Player/Tank/Abilities/Railgun/Cue_TankRailgunFire.Cue_TankRailgunFire" _cannonstaticmesh)
  (`KismetSystemLibrary.Delay` (`self.Charge Up Time`))
  (bind _returnvalue_2 (`GameplayStatics.SpawnEmitterAtLocation` "/Game/VFX/Abilities/Railgun/P_RailgunBeam.P_RailgunBeam" (`SceneComponent.K2_GetComponentLocation` _cannonstaticmesh)))
  (bind _returnvalue_3 (`SceneComponent.K2_GetComponentLocation` _cannonstaticmesh))
  (bind _output_get (set `self.Beam Collision Point` (+ (* (`KismetMathLibrary.GetForwardVector` (`SceneComponent.K2_GetComponentRotation` _cannonstaticmesh)) (`self.Railgun Length`)) _returnvalue_3)))
  ;;[0.5651 1 0.5198] CapsuleTrace Calculates Collision of Railgun, Sets VFX Target Point
  (bind (_outhit _returnvalue_4) (`KismetSystemLibrary.CapsuleTraceSingle` _returnvalue_3 _output_get 40.0 20.0 "TraceTypeQuery1" false (`|MakeArray` (`self.GetOwner`)) (`self.Railgun Trace Visibility`)))
  (if _returnvalue_4
    (bind (_bblockinghit _binitialoverlap _time _distance _location _impactpoint _normal _impactnormal _physmat _hitactor) (`GameplayStatics.BreakHitResult` _outhit))
    (bind _output_get_2 (set `self.Beam Collision Point` _impactpoint)))
  (`ParticleSystemComponent.SetBeamTargetPoint` _returnvalue_2 0 _output_get_2 0)
  (`KismetSystemLibrary.PrintString` (`KismetSystemLibrary.GetDisplayName` _hitactor) (`self.Print All Trace Hits`) false (struct :`G` 0.66 :`B` 1.0 :`A` 1.0) 0.5)
  ;;[0.9922 0.3191 1] TestPTank is TEMP
  (bind _astest_ptank (cast `/Game/Blueprints/Tanks/TestPTank` _hitactor))
  (bind _healthcomponent (`BaseTank.HealthComponent` _astest_ptank))
  ;;[1 0.1863 0.1664] Causes Damage to Enemy Tank If Hit
  (`HealthComponent.TakeDamage` _healthcomponent 1.0)
  (`/Game/Blueprints/Tanks/TestPTank.Trigger Damage States` _astest_ptank)
  (bind _returnvalue_5 (`HealthComponent.CheckDeath` _healthcomponent))
  (if _returnvalue_5
    (`KismetSystemLibrary.PrintString` "Tank Destroyed" _returnvalue false (struct :`G` 0.66 :`B` 1.0 :`A` 1.0) 1.0)
    (else
      (`KismetSystemLibrary.PrintString` "Damage!" _returnvalue false (struct :`G` 0.66 :`B` 1.0 :`A` 1.0) 1.0))))