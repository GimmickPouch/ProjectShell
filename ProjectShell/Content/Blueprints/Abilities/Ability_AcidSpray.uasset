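; Tank ability that sprays acid blobs from the cannon, leaving puddles that damage tanks over time.
; A delayed self-calling event launches randomly sized blobs by impulse until the maximum is reached.
; Puddles register in an array and are destroyed when the cooldown expires.
; Entering starts looping sound and a ticking damage loop, which leaving stops once no tracked puddle still overlaps the tank.
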(event `Clear Puddles`
  ;[0.1006 1 0] Wait for Cooldown to Expire, then Despawn All Acid Blobs.
  (for _array_element (`self.Active Acid Puddles`)
    (`Actor.K2_DestroyActor` _array_element))
  (`KismetArrayLibrary.Array_Clear` (`self.Active Acid Puddles`))
  (set `self.Active Blobs` 0)
  (`AudioComponent.FadeOut` (`self.SFX_Damage`) 0.15 0.0))

(event `Spawn Additional Blob`
  ;[0.7898 1 0.5198] Spawn Additional Acid Blobs
  (`KismetSystemLibrary.Delay` 0.2)
  (bind _cannonbase (`BaseTank.CannonBase` (stale `self.AbilityAction` _asbase_tank)))
  (bind _returnvalue (* (`KismetMathLibrary.GetForwardVector` (`SceneComponent.K2_GetComponentRotation` _cannonbase)) 200.0))
  ;[0.6049 1 0.3695] Spawn an Acid Spray Blob
  (bind _returnvalue_2 (`|SpawnActorFromClass` "/Game/Blueprints/Abilities/AbilityActors/AcidSprayBlob.AcidSprayBlob_C" (`KismetMathLibrary.MakeTransform` (+ (`SceneComponent.K2_GetComponentLocation` _cannonbase) _returnvalue) (struct) (`KismetMathLibrary.Conv_DoubleToVector` (`KismetMathLibrary.RandomFloatInRange` (`self.Minimum Blob Size`) (`self.Maximum Blob Size`)))) "Undefined" "OverrideRootScale" (`self.GetOwner`) null :!label _label))
  ;[1 0.7104 0.8923] Push Acid Blob Forwards
  (bind _asbase_tank (cast `BaseTank` (`self.GetOwner`)))
  (`PrimitiveComponent.AddImpulseAtLocation` (`/Game/Blueprints/Abilities/AbilityActors/AcidSprayBlob.Blob` _returnvalue_2) (* (`SceneComponent.GetForwardVector` (`BaseTank.CannonBase` _asbase_tank)) (`self.Blob Throw Force`)) _returnvalue "None")
  ;[0.5296 1 0.4679] Keep Track of Total Number of Acid Blobs, Spawn More If Necessary
  (bind _result (`/Engine/EditorBlueprintResources/StandardMacros.IncrementInt` (`self.Active Blobs`))
    (:`  `
      (bind _output_get (set `self.Active Blobs` _result))
      (if (not (>= _output_get (`self.Maximum Acid Spray Blobs`)))
        (`self.Spawn Additional Blob`)))))

(event `self.AbilityAction`
  ;[0.6049 1 0.3695] Spawn an Acid Spray Blob
  (`|ExecutionSequence`
    (:`then_0`
      (`KismetSystemLibrary.Delay` (`self.AbilityCooldownSeconds`))
      (`self.Clear Puddles`))
    (:`then_1`
      (bind _asbase_tank (cast `BaseTank` (`self.GetOwner`)))
      (`GameplayStatics.SpawnSoundAttached` "/Game/Audio/Player/Tank/Abilities/AcidSpray/Cue_AcidSprayFire.Cue_AcidSprayFire" (`BaseTank.CannonBase` _asbase_tank))
      (goto _label))))

(event `Tank Enters Puddle`
  (params (Tank :type "BaseTank Object Reference"))
  ;[1 0.2696 0.2497] Tank Enters Puddle and Takes Damage Every Tick
  (if (not (`self.Audio Playing`))
    (bind _returnvalue (`GameplayStatics.SpawnSoundAttached` "/Game/Audio/Player/Tank/Abilities/AcidSpray/Cue_AcidSprayDamage.Cue_AcidSprayDamage" (`BaseTank.CannonBase` Tank)))
    (set `self.SFX_Damage` _returnvalue)
    (set `self.Audio Playing` true))
  (`KismetSystemLibrary.Delay` (`self.Damage Tick`) :!label _label_2)
  (if (`self.Tank Taking Damage`)
    (bind _astest_ptank (cast `/Game/Blueprints/Tanks/TestPTank` Tank))
    (`HealthComponent.TakeDamage` (`BaseTank.HealthComponent` _astest_ptank) 1.0)
    (`/Game/Blueprints/Tanks/TestPTank.Trigger Damage States` _astest_ptank)
    (`self.Puddle Damages Tank`)))

(event `Add Puddle to Array`
  (params (Puddle :type "/Game/Blueprints/Abilities/AbilityActors/AcidSprayPuddle Object Reference"))
  ;[0.3904 0.4224 1] Add Puddle to an Array
  (`KismetArrayLibrary.Array_Add` (`self.Active Acid Puddles`) Puddle))

(event `Puddle Damages Tank`
  ;[1 0.2696 0.2497] Tank Enters Puddle and Takes Damage Every Tick
  (goto _label_2))

(fn `Tank Leaves Puddle`
  (params (Tank :type "BaseTank Object Reference"))
  (locals (`Tank Is Free` :type Boolean :default true))
  (bind _active_acid_puddles (`self.Active Acid Puddles`))
  ;[1 1 1] Tank Leaves Puddle, Called by Puddle End Overlap
  (if (!= (`KismetArrayLibrary.Array_Length` _active_acid_puddles) 0)
    (for _array_element _active_acid_puddles
      (if (`KismetArrayLibrary.Array_Contains` (`/Game/Blueprints/Abilities/AbilityActors/AcidSprayPuddle.Overlapping Tanks in Acid` _array_element) Tank)
        (set `local.Tank Is Free` false)
        (break))))
  (if (`local.Tank Is Free`)
    (set `self.Tank Taking Damage` false)
    (`AudioComponent.FadeOut` (`self.SFX_Damage`) 0.5 0.0)
    (set `self.Audio Playing` false)))