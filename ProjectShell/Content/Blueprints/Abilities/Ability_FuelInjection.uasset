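; Tank ability that grants a temporary fuel-injection speed boost to the owning BaseTank.
; When the ability action fires, it multiplies the tank's MoveSpeed by SpeedIncrease and plays an activation sound attached to the main body mesh.
; After a Duration delay, it divides MoveSpeed by the same factor to undo the boost, rather than restoring a cached value.
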(event `self.AbilityAction`
  (bind _asbase_tank (cast `BaseTank` (`self.GetOwner`)))
  (set `BaseTank.MoveSpeed` (* (`BaseTank.MoveSpeed` _asbase_tank) (`self.Speed Increase`)) _asbase_tank)
  (`GameplayStatics.SpawnSoundAttached` "/Game/Audio/Player/Tank/Abilities/FuelInjection/Cue_TankFuelActivate.Cue_TankFuelActivate" (`BaseTank.TankMainBodyMesh` _asbase_tank) "None" (`Actor.K2_GetActorLocation` _asbase_tank))
  (`KismetSystemLibrary.Delay` (`self.Duration`))
  (bind _asbase_tank_2 (cast `BaseTank` (`self.GetOwner`)))
  (set `BaseTank.MoveSpeed` (/ (`BaseTank.MoveSpeed` _asbase_tank_2) (`self.Speed Increase`)) _asbase_tank_2))