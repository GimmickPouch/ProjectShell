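; Toxic spill puddle weapon hazard that starts and stops a toxic damage countdown on tanks that overlap it.
; On BeginPlay it counts its owner TestTank as in a puddle (marked temporary), then a timeline delays arming.
; Once active, overlaps by actors of exactly BaseTank class that cast to TestTank adjust that tank's puddle count, clamped before incrementing.
; Countdown and damage logic live on the tank.
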(event `self.ReceiveBeginPlay`
  ;[1 1 1] Make Puddle Active
  (bind _astest_tank (cast `/Game/Blueprints/Tanks/TestTank` (`self.GetOwner`)))
  (set `/Game/Blueprints/Tanks/TestTank.Tank in Puddles` (+ (`/Game/Blueprints/Tanks/TestTank.Tank in Puddles` _astest_tank) 1) _astest_tank)
  (`TimelineComponent.SetPlayRate` (`self.Tank Check Timeline`) (/ 1.0 1.0))
  (`Timeline|Tank Check Timeline` :!via `PlayFromStart`
    (:`Finished`
      (if (not (`self.Active?`))
        (set `self.Active?` true)))))

(event `self.ReceiveActorBeginOverlap`
  (params (OtherActor :type "Actor Object Reference"))
  ;[1 1 1] Tank Moves Onto Puddle, Added to Puddle Total
  (if (`self.Active?`)
    (if (== (`GameplayStatics.GetObjectClass` OtherActor) "/Script/ProjectShell.BaseTank")
      (bind _astest_tank (cast `/Game/Blueprints/Tanks/TestTank` OtherActor))
      (`/Game/Blueprints/Tanks/TestTank.Toxic Countdown to Damage` _astest_tank)
      (set `/Game/Blueprints/Tanks/TestTank.Tank in Puddles` (+ (`KismetMathLibrary.Clamp` (`/Game/Blueprints/Tanks/TestTank.Tank in Puddles` _astest_tank) 0 (* (`/Game/Blueprints/Tanks/TestTank.Number of Toxic Spill Puddles` _astest_tank) 4)) 1) _astest_tank))))

(event `self.ReceiveActorEndOverlap`
  (params (OtherActor :type "Actor Object Reference"))
  ;[1 1 1] Tank Moves Away, Removed from Puddle Total
  (if (`self.Active?`)
    (if (== (`GameplayStatics.GetObjectClass` OtherActor) "/Script/ProjectShell.BaseTank")
      (bind _astest_tank (cast `/Game/Blueprints/Tanks/TestTank` OtherActor))
      (`/Game/Blueprints/Tanks/TestTank.Stop Toxic Countdown` _astest_tank)
      (set `/Game/Blueprints/Tanks/TestTank.Tank in Puddles` (- (`/Game/Blueprints/Tanks/TestTank.Tank in Puddles` _astest_tank) 1) _astest_tank))))

(fn `UserConstructionScript`)