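; Test tank Blueprint with an experimental dual-cannon mode and health-based damage feedback.
; Gamepad top face button toggles cannon meshes, fire rate and spawn offset; a self-calling delayed event alternates barrels on time, not per shot.
; Projectile hits, or debug key J damage, print health and update team-colored materials, smoke and damage sounds from HealthComponent's value.
; The PreDeath override plays an explosion sound.
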(event `Looping Bullet Offset`
  ;[0.2893 0.6615 0.2417] DualCannon Experiment - Still Needs Reduced Damage and / or Range
  ;;[1 1 1] Should Toggle on Fire, Not Time
  (`KismetSystemLibrary.Delay` 0.4)
  (if (`self.Enable TwoShot`)
    (if (== (`self.BulletSpawnOffset`) (120.0 30.0 0.0) :`ErrorTolerance` 0.1)
      (set `self.BulletSpawnOffset` (120.0 -30.0 0.0))
      (else
        (set `self.BulletSpawnOffset` (120.0 30.0 0.0))))
    (`self.Looping Bullet Offset`)))

(event `Key|Gamepad_FaceButton_Top`
  (params (Key :type "Key Structure"))
  ;[0.2893 0.6615 0.2417] DualCannon Experiment - Still Needs Reduced Damage and / or Range
  (:`Pressed`
    (if (`self.Enable TwoShot`)
      (set `self.Enable TwoShot` false)
      (set `self.BulletSpawnOffset` (120.0 0.0 0.0))
      (set `self.FireRate` 1.0)
      (`SceneComponent.SetVisibility` (`self.CannonStaticMesh`) true false)
      (`SceneComponent.SetVisibility` (`self.DualCannonL`) false false)
      (`SceneComponent.SetVisibility` (`self.DualCannonR`) false false)
      (else
        (set `self.Enable TwoShot` true)
        (set `self.BulletSpawnOffset` (120.0 30.0 0.0))
        (set `self.FireRate` 0.3)
        (`SceneComponent.SetVisibility` (`self.CannonStaticMesh`) false false)
        (`SceneComponent.SetVisibility` (`self.DualCannonL`) true false)
        (`SceneComponent.SetVisibility` (`self.DualCannonR`) true false)
        (`self.Looping Bullet Offset`)))))

(event `self.PreDeath`
  ;[0.3125 0.207 0.1232] Override PreDeath, Play Explosion VFX / SFX
  (`GameplayStatics.PlaySoundAtLocation` "/Game/Audio/Player/Tank/Damage/Death/Cue_TankDieExplode.Cue_TankDieExplode" (`self.K2_GetActorLocation`)))

(event `Key|J`
  (params (Key :type "Key Structure"))
  (bind _healthcomponent (`self.HealthComponent`))
  ;[0.5208 0.2942 0.3359] Tank Damage
  (:`Pressed`
    (`HealthComponent.TakeDamage` _healthcomponent 1.0)
    (bind _returnvalue (`HealthComponent.CheckDeath` _healthcomponent))
    (if (not _returnvalue)
      (`KismetSystemLibrary.PrintString` (`KismetStringLibrary.Conv_DoubleToString` (`HealthComponent.GetHealth` (`self.HealthComponent`))) :!label _label)
      (`self.Trigger Damage States`))))

(event `self.ReceiveHit`
  (params (MyComp :type "PrimitiveComponent Object Reference") (Other :type "Actor Object Reference") (OtherComp :type "PrimitiveComponent Object Reference") (bSelfMoved :type Boolean) (HitLocation :type "Vector Structure") (HitNormal :type "Vector Structure") (NormalImpulse :type "Vector Structure") (Hit :type "HitResult Structure (by ref)"))
  ;[0.5208 0.2942 0.3359] Tank Damage
  (cast `BaseProjectile` Other)
  (`KismetSystemLibrary.Delay` 0.01)
  (goto _label))

(event `Trigger Damage States`
  (bind _tankmainbodymesh (`self.TankMainBodyMesh`))
  (bind _tankmainbodymesh_2 (`self.TankMainBodyMesh`))
  (bind _returnvalue (`HealthComponent.GetHealth` (`self.HealthComponent`)))
  (bind _returnvalue_2 (`PrimitiveComponent.GetMaterial` (`self.TankMainBodyMesh`) 0))
  ;[1 1 1] Trigger Damage States
  (if (== _returnvalue 3.0)
    (if (== (`PrimitiveComponent.GetMaterial` (`self.TankMainBodyMesh`) 0) "/Game/Geometry/Materials/M_TankBlueDamaged.M_TankBlueDamaged")
      (`PrimitiveComponent.SetMaterial` _tankmainbodymesh 0 "/Game/Geometry/Materials/M_TankBlue.M_TankBlue")
      (else
        (`PrimitiveComponent.SetMaterial` _tankmainbodymesh 0 "/Game/Geometry/Materials/M_TankRed.M_TankRed")))
    (`ActorComponent.Deactivate` (`self.Smoke`))
    (elif (== _returnvalue 2.0)
      (if (or (== _returnvalue_2 "/Game/Geometry/Materials/M_TankBlueDamaged.M_TankBlueDamaged") (== _returnvalue_2 "/Game/Geometry/Materials/M_TankBlue.M_TankBlue"))
        (`PrimitiveComponent.SetMaterial` _tankmainbodymesh_2 0 "/Game/Geometry/Materials/M_TankBlueDamaged.M_TankBlueDamaged")
        (else
          (`PrimitiveComponent.SetMaterial` _tankmainbodymesh_2 0 "/Game/Geometry/Materials/M_TankRedDamaged.M_TankRedDamaged")))
      (`AudioComponent.Play` (`self.Cue_TankDamageLight`) 0.0)
      (`ActorComponent.Deactivate` (`self.Smoke`))
      (elif (== _returnvalue 1.0)
        (`ActorComponent.Activate` (`self.Smoke`) false)
        (`AudioComponent.Play` (`self.Cue_TankDamageHeavy`) 0.0)))))

(fn `UserConstructionScript`)