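; TestTank is a prototype tank with team-coloured cannon meshes, a health readout and two cooldown-limited abilities.
; HealthComponent feeds the text display, refreshed on Hit after a brief delay, while a Backspace debug key deals damage and destroys the tank on death.
; The railgun special briefly makes a placeholder beam visible and overlapping.
; The defensive blink sweeps the tank forward, starting its cooldown only if the move succeeds.
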(event `Set Tank Team Colour`
  (bind __cannonstaticmesh (`self._cannonStaticMesh`))
  ;[1 1 1] Tank Barrel Colouring
  (if (`self.Team Toggle`)
    (`PrimitiveComponent.SetMaterial` __cannonstaticmesh 0 "/Game/TwinStick/Meshes/BlueMaterial.BlueMaterial")
    (`PrimitiveComponent.SetMaterial` (`self._cannonBaseStaticMesh`) 0 "/Game/TwinStick/Meshes/BlueMaterial.BlueMaterial")
    (else
      (`PrimitiveComponent.SetMaterial` __cannonstaticmesh 0 "/Game/TwinStick/Meshes/RedMaterial.RedMaterial")
      (`PrimitiveComponent.SetMaterial` (`self._cannonBaseStaticMesh`) 0 "/Game/TwinStick/Meshes/RedMaterial.RedMaterial"))))

(event `self.ReceiveHit`
  (params (MyComp :type "PrimitiveComponent Object Reference") (Other :type "Actor Object Reference") (OtherComp :type "PrimitiveComponent Object Reference") (bSelfMoved :type Boolean) (HitLocation :type "Vector Structure") (HitNormal :type "Vector Structure") (NormalImpulse :type "Vector Structure") (Hit :type "HitResult Structure (by ref)"))
  ;[1 1 1] Set HP Display
  (`KismetSystemLibrary.Delay` 0.01)
  (`TextRenderComponent.K2_SetText` (`self.DisplayHealth`) (`KismetTextLibrary.Conv_DoubleToText` (`HealthComponent.GetHealth` (`self._healthComponent`)) "HalfToEven") :!label _label))

(event `Key|BackSpace`
  (params (Key :type "Key Structure"))
  ;[1 1 1] Set HP Display
  (:`Pressed`
    (bind _returnvalue (`HealthComponent.TakeDamageAndCheckDeath` (`self._healthComponent`) 1.0))
    (if _returnvalue
      (`self.K2_DestroyActor`)
      (else
        (goto _label)))))

(event `self.ReceiveBeginPlay`
  ;[1 1 1] Set HP Display
  (`TextRenderComponent.K2_SetText` (`self.DisplayHealth`) (`KismetTextLibrary.Conv_DoubleToText` (`HealthComponent.GetHealth` (`self._healthComponent`)) "HalfToEven"))
  ;[1 1 1] Railgun needs to start with no collision
  (`PrimitiveComponent.SetCollisionResponseToAllChannels` (`self.TEMPRailgunBeam`) "ECR_Ignore"))

(event `self.SpecialAbilityAction`
  (bind _temprailgunbeam (`self.TEMPRailgunBeam`))
  (bind _temprailgunbeam_2 (`self.TEMPRailgunBeam`))
  ;[1 1 1] Special Ability Prototype - Railgun
  (if (not (`self.Special On Cooldown`))
    (`PrimitiveComponent.SetCollisionResponseToAllChannels` _temprailgunbeam "ECR_Overlap")
    (`SceneComponent.SetVisibility` _temprailgunbeam true false)
    (set `self.Special On Cooldown` true)
    (`KismetSystemLibrary.Delay` 0.2)
    (`PrimitiveComponent.SetCollisionResponseToAllChannels` _temprailgunbeam_2 "ECR_Ignore")
    (`SceneComponent.SetVisibility` _temprailgunbeam_2 false false)
    (`KismetSystemLibrary.Delay` 3.5)
    (set `self.Special On Cooldown` false)))

(event `self.DefensiveAbilityAction`
  ;[1 1 1] Defensive Ability Prototype - Blink
  (if (not (`self.Defensive On Cooldown`))
    (bind (_sweephitresult _returnvalue) (`self.K2_SetActorLocation` (+ (* (`self.GetActorForwardVector`) (`self.Teleport Range`)) (`self.K2_GetActorLocation`)) true))
    (if _returnvalue
      ;;[1 1 1] Unused VFX
      (`GameplayStatics.SpawnEmitterAtLocation` null)
      (set `self.Defensive On Cooldown` true)
      (`KismetSystemLibrary.Delay` 4.0)
      (set `self.Defensive On Cooldown` false))))

(fn `UserConstructionScript`)