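; TriggerFloor is a floor pressure button that reacts to TestTank actors.
; When a TestTank begins overlapping, it teleports the TriggerButtonSM component 10 units down and sets Triggered to true.
; When one stops overlapping, it raises the button again and clears Triggered.
; The class check is an exact match, and overlaps are not counted, so each tank entering or leaving moves the button.
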(event `self.ReceiveActorBeginOverlap`
  (params (OtherActor :type "Actor Object Reference"))
  (if (== (`GameplayStatics.GetObjectClass` OtherActor) "/Game/Blueprints/Tanks/TestTank.TestTank_C")
    (`SceneComponent.K2_AddLocalOffset` (`self.TriggerButtonSM`) (0.0 0.0 -10.0) false true)
    (set `self.Triggered?` true)))

(event `self.ReceiveActorEndOverlap`
  (params (OtherActor :type "Actor Object Reference"))
  (if (== (`GameplayStatics.GetObjectClass` OtherActor) "/Game/Blueprints/Tanks/TestTank.TestTank_C")
    (`SceneComponent.K2_AddLocalOffset` (`self.TriggerButtonSM`) (0.0 0.0 10.0) false true)
    (set `self.Triggered?` false)))

(fn `UserConstructionScript`)