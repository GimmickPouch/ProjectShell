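; HazardSawblade is an environmental hazard that slides back and forth and kills a TestTank on overlap.
; The overlap deals lethal-scale damage through the tank's HealthComponent, then destroys it as a temporary workaround for broken death handling.
; A Timeline, rate-scaled by a duration variable, sweeps the blade between its start location and an absolute world X set by ReturnDistance.
; It reverses when playback stops and restarts once back at the start.
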(event `self.ReceiveActorBeginOverlap`
  (params (OtherActor :type "Actor Object Reference"))
  ;[1 1 1] Sawblade Causes Damage
  (if (== (`GameplayStatics.GetObjectClass` OtherActor) "/Game/Blueprints/Tanks/TestTank.TestTank_C")
    (bind _astest_tank (cast `/Game/Blueprints/Tanks/TestTank` OtherActor))
    (`HealthComponent.TakeDamage` (`BaseTank._healthComponent` _astest_tank) 1000.0)
    ;[1 1 1] To Be Removed When Death is Fixed
    (`self.K2_DestroyActor` _astest_tank)))

(event `self.ReceiveBeginPlay`
  ;[1 1 1] Sawblade Movement
  ;;[1 0.956 0.5979] Sawmill Loop
  (set `self.StartPosition` (`self.K2_GetActorLocation`))
  (`TimelineComponent.SetPlayRate` (`self.SawbladeMoveDuration`) (/ 1.0 (`self.Sawblade Move Duration`)))
  (bind (_direction _alpha) (`Timeline|SawbladeMoveDuration` :!label _label)
    (:`Update`
      ;;[0.4143 1 0.6242] Play, then Reverse when Finished
      (`self.K2_SetActorLocation` (`KismetMathLibrary.VLerp` (`self.StartPosition`) (`KismetMathLibrary.MakeVector` (`self.Return Distance`) (.y (`self.StartPosition`)) (.z (`self.StartPosition`))) _alpha) true)
      (if (not (`TimelineComponent.IsPlaying` (`self.SawbladeMoveDuration`)))
        (`TimelineComponent.Reverse` (`self.SawbladeMoveDuration`))))
    (:`Finished`
      (if (== (`self.StartPosition`) (`self.K2_GetActorLocation`))
        (goto _label :!via `PlayFromStart`)))))

(fn `UserConstructionScript`)