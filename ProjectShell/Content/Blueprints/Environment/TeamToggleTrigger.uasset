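; Trigger actor that colours a tank's cannon by team, based on its starting position.
; On overlap, the BlueTeam boolean selects the blue or red material for the BaseTank's cannon mesh.
; Each branch's DoOnce precedes the class check, so the first overlapping actor of any class uses it up.
; Actual team-toggle logic is still a placeholder awaiting code; only the material changes.
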(event `self.ReceiveActorBeginOverlap`
  (params (OtherActor :type "Actor Object Reference"))
  ;[1 1 1] Sets Tank Turret to Team Colour Based on Starting Position. Set "Blue Team?" Boolean to Dictate Colours
  (if (`self.Blue Team?`)
    ;;[0.06901 0.003043 1] True for Blue Team
    (`/Engine/EditorBlueprintResources/StandardMacros.DoOnce` false
      (:`Completed`
        (if (`KismetMathLibrary.ClassIsChildOf` (`GameplayStatics.GetObjectClass` OtherActor) "/Script/ProjectShell.BaseTank")
          (bind _asbase_tank (cast `BaseTank` OtherActor))
          ;;;[1 1 1] Need Team Toggle Logic - Wait For Code
          (`PrimitiveComponent.SetMaterial` (`BaseTank.CannonStaticMesh` _asbase_tank) 0 "/Game/TwinStick/Meshes/BlueMaterial.BlueMaterial"))))
    (else
      ;;[1 0 0.01909] False for Red Team
      (`/Engine/EditorBlueprintResources/StandardMacros.DoOnce` false
        (:`Completed`
          (if (`KismetMathLibrary.ClassIsChildOf` (`GameplayStatics.GetObjectClass` OtherActor) "/Script/ProjectShell.BaseTank")
            (bind _asbase_tank_2 (cast `BaseTank` OtherActor))
            ;;;[1 1 1] Need Team Toggle Logic - Wait For Code
            (`PrimitiveComponent.SetMaterial` (`BaseTank.CannonStaticMesh` _asbase_tank_2) 0 "/Game/TwinStick/Meshes/RedMaterial.RedMaterial")))))))

(fn `UserConstructionScript`)