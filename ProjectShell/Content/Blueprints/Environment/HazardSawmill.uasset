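; A moving sawblade hazard that kills a TestTank on overlap.
; The overlap deals massive damage through the tank's HealthComponent, then destroys the actor as a temporary workaround for broken death handling.
; On BeginPlay, a timeline lerps the blade with sweep from its start position to the ReturnPosition actor, then reverses.
; The loop is unfinished: nothing replays the timeline forward after the return trip.
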(event `self.ReceiveActorBeginOverlap`
  (params (OtherActor :type "Actor Object Reference"))
  ;[1 1 1] Sawblade Causes Damage
  (if (== (`GameplayStatics.GetObjectClass` OtherActor) "/Game/Blueprints/Tanks/TestTank.TestTank_C")
    (bind _astest_tank (cast `/Game/Blueprints/Tanks/TestTank` OtherActor))
    (`HealthComponent.TakeDamage` (`BaseTank._healthComponent` _astest_tank) 1000.0)
    ;[1 1 1] To Be Removed When Death is Fixed
    (`self.K2_DestroyActor` _astest_tank)))

(event `self.ReceiveBeginPlay`
  ;[1 1 1] Unfinished Loop
  (set `self.StartPosition` (`self.K2_GetActorLocation`))
  (bind (_direction _alpha) (`Timeline|MoveBetweenPoints` :!label _label)
    (:`Update`
      (`self.K2_SetActorLocation` (`KismetMathLibrary.VLerp` (`self.StartPosition`) (`self.K2_GetActorLocation` (`self.ReturnPosition`)) _alpha) true))
    (:`Finished`
      (goto _label :!via `Reverse`))))

(fn `UserConstructionScript`)