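; RepairKit is a pickup that heals an overlapping BaseTank by one health point, without overheal, if it is not at max health.
; It plays a sound, refreshes damage states via a TestPTank cast, then hides and either respawns after a cooldown or destroys itself.
; A failed TestPTank cast leaves the kit active after healing.
; Tick spins the wrench mesh by a fixed yaw step per frame.
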(event `self.ReceiveActorBeginOverlap`
  (params (OtherActor :type "Actor Object Reference"))
  ;[1 1 1] Tank Picks Up Repair Kit
  (bind _asbase_tank (cast `BaseTank` OtherActor))
  (bind _healthcomponent (`BaseTank.HealthComponent` _asbase_tank))
  (if (not (== (`HealthComponent.GetHealth` _healthcomponent) (`HealthComponent.GetMaxHealth` _healthcomponent)))
    (`HealthComponent.IncreaseHealth` _healthcomponent 1.0 false)
    (`GameplayStatics.PlaySoundAtLocation` "/Game/Audio/Items/RepairKit/Cue_RepairKitPickup.Cue_RepairKitPickup" (`self.K2_GetActorLocation`))
    (bind _astest_ptank (cast `/Game/Blueprints/Tanks/TestPTank` _asbase_tank))
    (`/Game/Blueprints/Tanks/TestPTank.Trigger Damage States` _astest_ptank)
    (`self.SetActorEnableCollision` false)
    (`self.SetActorHiddenInGame` true)
    (if (`self.Able to Respawn`)
      ;[1 1 1] Repair Kit Cooldown and Reset
      (`KismetSystemLibrary.Delay` (`self.Repair Kit Cooldown`))
      (`self.SetActorEnableCollision` true)
      (`self.SetActorHiddenInGame` false)
      (`GameplayStatics.PlaySoundAtLocation` "/Game/Audio/Items/RepairKit/Cue_RepairKitRespawn.Cue_RepairKitRespawn" (`self.K2_GetActorLocation`))
      (else
        (`self.K2_DestroyActor`)))))

(event `self.ReceiveTick`
  (params (DeltaSeconds :type "Float (single-precision)"))
  (bind _smwrench (`self.SMWrench`))
  ;[1 1 1] Repair Kit Spins
  (`SceneComponent.K2_SetRelativeRotation` _smwrench (`KismetMathLibrary.MakeRotator` (.roll (`SceneComponent.RelativeRotation` _smwrench)) (.pitch (`SceneComponent.RelativeRotation` _smwrench)) (+ (.yaw (`SceneComponent.RelativeRotation` _smwrench)) 1.0)) false false))

(fn `UserConstructionScript`)